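; Inventory component that tracks money and per-type counts of seeds and plants, likely for a farming or gardening game.
; Add and subtract functions update the Seeds and Plants maps or Money, then fire change dispatchers for listeners.
; Only TrySubMoney checks the balance first; seed and plant subtraction is unguarded, with separate query functions available.
; Money changes play 2D sounds, with the gain sound on spending and the lose sound on adding.
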(fn `AddMoney`
  (params (Amount :type Integer))
  (set `self.Money` (+ (`self.Money`) Amount))
  (`GameplayStatics.PlaySound2D` "/Game/Audio/MS_LooseMoney.MS_LooseMoney" 1.0 1.0 0.0 null null)
  (`self.OnMoneyAmountChanged` (`self.Money`)))

(fn `AddPlants`
  (params (Plant :type "GameplayTag Structure") (Amount :type Integer))
  (bind _plant (`local.Plant`))
  (bind (_value _returnvalue) (`BlueprintMapLibrary.Map_Find` (`self.Plants`) Plant))
  (`BlueprintMapLibrary.Map_Add` (`self.Plants`) Plant (+ Amount (`KismetMathLibrary.SelectInt` _value 0 _returnvalue)))
  (`self.OnPlantAmountChanged` _plant (`BlueprintMapLibrary.Map_Find` (`self.Plants`) _plant)))

(fn `AddSeeds`
  (params (Seed :type "GameplayTag Structure") (Amount :type Integer))
  (bind _seed (`local.Seed`))
  (bind (_value _returnvalue) (`BlueprintMapLibrary.Map_Find` (`self.Seeds`) Seed))
  (`BlueprintMapLibrary.Map_Add` (`self.Seeds`) Seed (+ Amount (`KismetMathLibrary.SelectInt` _value 0 _returnvalue)))
  (`self.OnSeedAmountChanged` _seed (`BlueprintMapLibrary.Map_Find` (`self.Seeds`) _seed)))

(fn `CanSpendMoney`
  (params (Amount :type Integer))
  (returns (ReturnValue :type Boolean))
  (return (>= (`self.Money`) Amount)))

(fn `CanSpendPlants`
  (params (Plant :type "GameplayTag Structure") (Amount :type Integer))
  (returns (ReturnValue :type Boolean))
  (bind (_value _returnvalue) (`BlueprintMapLibrary.Map_Find` (`self.Plants`) Plant))
  (if _returnvalue
    (return (>= _value Amount))
    (else
      (return false))))

(fn `Has Plant`
  (params (Plant :type "GameplayTag Structure"))
  (returns (ReturnValue :type Boolean))
  (return (> (`BlueprintMapLibrary.Map_Find` (`self.Plants`) Plant) 0)))

(fn `HasMoney`
  (returns (ReturnValue :type Boolean))
  (return (> (`self.Money`) 0)))

(fn `HasSeed`
  (params (Seed :type "GameplayTag Structure"))
  (returns (ReturnValue :type Boolean))
  (return (> (`BlueprintMapLibrary.Map_Find` (`self.Seeds`) Seed) 0)))

(fn `SubPlants`
  (params (Plant :type "GameplayTag Structure") (Amount :type Integer))
  (bind _plant (`local.Plant`))
  (`BlueprintMapLibrary.Map_Add` (`self.Plants`) Plant (- (`BlueprintMapLibrary.Map_Find` (`self.Plants`) Plant) Amount))
  (`self.OnPlantAmountChanged` _plant (`BlueprintMapLibrary.Map_Find` (`self.Plants`) _plant)))

(fn `SubSeed`
  (params (Seed :type "GameplayTag Structure") (Amount :type Integer))
  (bind _seed (`local.Seed`))
  (bind _seeds (`self.Seeds`))
  (`BlueprintMapLibrary.Map_Add` _seeds Seed (- (`BlueprintMapLibrary.Map_Find` _seeds Seed) Amount))
  (`self.OnSeedAmountChanged` _seed (`BlueprintMapLibrary.Map_Find` (`self.Seeds`) _seed)))

(fn `TrySubMoney`
  (params (Amount :type Integer))
  (returns (bSuccess :type Boolean))
  (if (`self.CanSpendMoney` Amount)
    (set `self.Money` (- (`self.Money`) Amount))
    (`GameplayStatics.PlaySound2D` "/Game/Audio/MS_GainMoney.MS_GainMoney" 1.0 1.0 0.0 null null)
    (`self.OnMoneyAmountChanged` (`self.Money`))
    (return true)
    (else
      (return false))))