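; Component that lets its owning actor carry one carrieable item at a time, with pickup, release and class-filtered lookup.
; PickUp attaches the item's owner to a left or right socket on an injected mesh, applies any custom attach transform and fires pickup events on both sides.
; LetGo detaches it, then either destroys it or line-traces down from the socket to place it on the floor.
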(fn `GetCurrentCarrieable`
  (returns (Carrieable :type "/Game/Gameplay/BPC_Carrieable Object Reference") (CarrieableOwner :type "Actor Object Reference"))
  (bind _carrieditem (`self.CarriedItem`))
  (return _carrieditem (`self.GetOwner` _carrieditem)))

(fn `GetSocket`
  (returns (Socket :type Name))
  (return (`KismetMathLibrary.SelectName` (`self.SocketNameR`) (`self.SocketNameL`) (`/Game/Gameplay/BPC_Carrieable.bUseRightHand` (`self.CarriedItem`)))))

(fn `InjectDependencies`
  (params (CarrierMesh :type "SkeletalMeshComponent Object Reference"))
  (set `self.CarrierMesh` CarrierMesh))

(fn `IsCarrying`
  (returns (ReturnValue :type Boolean))
  (return (`KismetSystemLibrary.IsValid` (`self.CarriedItem`))))

(fn `LetGo`
  (params (bDestroyCarrieable :type Boolean))
  (`/Engine/EditorBlueprintResources/StandardMacros.IsValid` (`self.CarriedItem`)
    (:`Is Valid`
      (`Actor.K2_DetachFromActor` (`self.GetOwner` (`self.CarriedItem`)) "KeepWorld" "KeepWorld" "KeepRelative")
      (if bDestroyCarrieable
        (`Actor.K2_DestroyActor` (`self.GetOwner` (`self.CarriedItem`)))
        (else
          (`self.TeleportMeshToFloor`)))
      (set `self.CarriedItem` null))))

(fn `PickUp`
  (params (Carrieable :type "/Game/Gameplay/BPC_Carrieable Object Reference"))
  (bind _carrieditem (`self.CarriedItem`))
  (set `self.CarriedItem` Carrieable)
  (`self.SetCollision` false)
  (`Actor.K2_AttachToComponent` (`self.GetOwner` (`self.CarriedItem`)) (`self.CarrierMesh`) (`self.GetSocket`) "SnapToTarget" "SnapToTarget" "KeepRelative" false)
  (if (`/Game/Gameplay/BPC_Carrieable.bUseAttachTransform` (`self.CarriedItem`))
    (`Actor.K2_SetActorRelativeTransform` (`self.GetOwner` (`self.CarriedItem`)) (`/Game/Gameplay/BPC_Carrieable.AttachTransform` (`self.CarriedItem`)) false false))
  (`self.OnPickedUp` self _carrieditem)
  (`/Game/Gameplay/BPC_Carrieable.OnPickedUp` _carrieditem))

(fn `SetCollision`
  (params (bEnabled :type Boolean))
  (`PrimitiveComponent.SetCollisionResponseToChannel` (`self.CarrierMesh`) "ECC_GameTraceChannel1" (select `bool` bEnabled :`false` "ECR_Block" :`true` "ECR_Ignore" :!type "ECollisionResponse Enum")))

(fn `TeleportMeshToFloor`
  (bind _returnvalue (`SceneComponent.GetSocketLocation` (`self.CarrierMesh`) (`self.GetSocket`)))
  (bind _outhit (`KismetSystemLibrary.LineTraceSingle` _returnvalue (- _returnvalue (0.0 0.0 1000.0)) "TraceTypeQuery1" true (`|MakeArray` (`self.GetOwner`))))
  (`Actor.K2_SetActorLocation` (`self.GetOwner` (`self.CarriedItem`)) (`.ImpactPoint` (`GameplayStatics.BreakHitResult` _outhit)) false false)
  (`Actor.K2_SetActorRotation` (`self.GetOwner` (`self.CarrierMesh`)) (`KismetMathLibrary.MakeRotator` 0.0 0.0 (.yaw (`Actor.K2_GetActorRotation` (`self.GetOwner` (`self.CarrierMesh`))))) false))

(fn `TryGetCurrentCarrieable`
  (returns (Carrieable :type "/Game/Gameplay/BPC_Carrieable Object Reference") (`Carrieable Owner` :type "Actor Object Reference") (bFound :type Boolean))
  (bind _carrieditem (`self.CarriedItem`)
    (:`then`
      (return _carrieditem (`self.GetOwner` _carrieditem) true))
    (:`else`
      (return null null false))))

(fn `TryGetCurrentCarrieableFiltered`
  (params (FilterClass :type "Actor Class Reference"))
  (returns (Carrieable :type "/Game/Gameplay/BPC_Carrieable Object Reference") (CarrieableOwner :type "Actor Object Reference") (bFound :type Boolean))
  (bind (_carrieable _carrieable_owner _bfound) (`self.TryGetCurrentCarrieable`))
  (if _bfound
    (if (== (`GameplayStatics.GetObjectClass` _carrieable_owner) (`local.FilterClass`))
      (return _carrieable _carrieable_owner true)
      (else
        _)))
  (return _carrieable _carrieable_owner false))