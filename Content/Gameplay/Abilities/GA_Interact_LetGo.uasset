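; Gameplay ability that makes the player character let go of what it is carrying.
; Activation calls LetGo on the character's BPC_Carrier component, then ends the ability immediately.
; It can activate only when that component exists and reports that it is carrying.
; Both graphs look up player character 0 directly instead of using the ability's actor info.
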(event `self.K2_ActivateAbility`
  (`parent.K2_ActivateAbility`)
  (`/Game/Gameplay/BPC_Carrier.LetGo` (`Actor.GetComponentByClass` (`GameplayStatics.GetPlayerCharacter` 0) "/Game/Gameplay/BPC_Carrier.BPC_Carrier_C") false)
  (`self.K2_EndAbility`))

(fn `K2_CanActivateAbility`
  (params (ActorInfo :type "GameplayAbilityActorInfo Structure") (Handle :type "GameplayAbilitySpecHandle Structure"))
  (returns (RelevantTags :type "GameplayTagContainer Structure") (ReturnValue :type Boolean))
  (bind _returnvalue (`Actor.GetComponentByClass` (`GameplayStatics.GetPlayerCharacter` 0) "/Game/Gameplay/BPC_Carrier.BPC_Carrier_C"))
  (`parent.K2_CanActivateAbility` ActorInfo Handle)
  (`/Engine/EditorBlueprintResources/StandardMacros.IsValid` _returnvalue
    (:`Is Valid`
      (return (struct) (`/Game/Gameplay/BPC_Carrier.IsCarrying` _returnvalue)))
    (:`Is Not Valid`
      (return (struct) false))))