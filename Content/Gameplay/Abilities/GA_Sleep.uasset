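; Gameplay ability that makes the avatar sleep at the closest bed.
; Activation is allowed only when a closest-bed search from the avatar finds a valid result, with the parent check's result left unused.
; On activation it finds the closest actor with a bed component, calls Sleep on that component and ends immediately.
; The check also filters by the bed actor class, while activation searches by component class alone.
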(event `self.K2_ActivateAbility`
  (`parent.K2_ActivateAbility`)
  (`/Game/Gameplay/BPC_Bed.Sleep` (`Actor.GetComponentByClass` (`/Game/Gameplay/Abilities/BFL_ClosestSearches.Get Closest Actor with Component` (`self.GetAvatarActorFromActorInfo`) "/Game/Gameplay/BPC_Bed.BPC_Bed_C") "/Game/Gameplay/BPC_Bed.BPC_Bed_C"))
  (`self.K2_EndAbility`))

(fn `K2_CanActivateAbility`
  (params (ActorInfo :type "GameplayAbilityActorInfo Structure") (Handle :type "GameplayAbilitySpecHandle Structure"))
  (returns (RelevantTags :type "GameplayTagContainer Structure") (ReturnValue :type Boolean))
  (`parent.K2_CanActivateAbility` ActorInfo Handle)
  (return (struct) (`KismetSystemLibrary.IsValid` (`/Game/Gameplay/Abilities/BFL_ClosestSearches.Get Closest with Component` (`self.GetAvatarActorFromActorInfo`) "/Game/Gameplay/BP_Bed.BP_Bed_C" "/Game/Gameplay/BPC_Bed.BPC_Bed_C"))))