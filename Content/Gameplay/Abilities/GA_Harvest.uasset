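; Gameplay ability that harvests the closest grow spot and adds one of the resulting plant to the avatar's inventory.
; Activation is allowed only when a closest actor with BPC_GrowSpot exists and reports ready for harvest; the parent check's boolean result is ignored.
; On activation it repeats the search, calls Harvest, passes the result to BPC_Inventory and ends immediately.
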(event `self.K2_ActivateAbility`
  (bind _plant_tag (`/Game/Gameplay/BPC_GrowSpot.Harvest` (`Actor.GetComponentByClass` (`/Game/Gameplay/Abilities/BFL_ClosestSearches.Get Closest Actor with Component` (`self.GetAvatarActorFromActorInfo`) "/Game/Gameplay/BPC_GrowSpot.BPC_GrowSpot_C") "/Game/Gameplay/BPC_GrowSpot.BPC_GrowSpot_C")))
  (`/Game/Gameplay/BPC_Inventory.AddPlants` (`Actor.GetComponentByClass` (`self.GetAvatarActorFromActorInfo`) "/Game/Gameplay/BPC_Inventory.BPC_Inventory_C") _plant_tag 1)
  (`self.K2_EndAbility`))

(fn `K2_CanActivateAbility`
  (params (ActorInfo :type "GameplayAbilityActorInfo Structure") (Handle :type "GameplayAbilitySpecHandle Structure"))
  (returns (RelevantTags :type "GameplayTagContainer Structure") (ReturnValue :type Boolean))
  (bind _returnvalue (`/Game/Gameplay/Abilities/BFL_ClosestSearches.Get Closest Actor with Component` (`self.GetAvatarActorFromActorInfo`) "/Game/Gameplay/BPC_GrowSpot.BPC_GrowSpot_C"))
  (bind _relevanttags (`parent.K2_CanActivateAbility` ActorInfo Handle))
  (`/Engine/EditorBlueprintResources/StandardMacros.IsValid` _returnvalue
    (:`Is Valid`
      (return _relevanttags (`/Game/Gameplay/BPC_GrowSpot.IsReadyForHarvest` (`Actor.GetComponentByClass` _returnvalue "/Game/Gameplay/BPC_GrowSpot.BPC_GrowSpot_C"))))
    (:`Is Not Valid`
      (return (struct) false))))