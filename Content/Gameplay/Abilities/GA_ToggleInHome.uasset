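; Gameplay ability that toggles the avatar in or out of a home through the nearest door.
; Activation is allowed only when a closest-search from the avatar finds a valid BP_Door with a BPC_Door component.
; On activation it finds the closest actor with BPC_Door, calls that component's ToggleInside with the avatar, then ends immediately.
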(event `self.K2_ActivateAbility`
  (bind _returnvalue (`self.GetAvatarActorFromActorInfo`))
  (`parent.K2_ActivateAbility`)
  (`/Game/Gameplay/BPC_Door.ToggleInside` (`Actor.GetComponentByClass` (`/Game/Gameplay/Abilities/BFL_ClosestSearches.Get Closest Actor with Component` _returnvalue "/Game/Gameplay/BPC_Door.BPC_Door_C") "/Game/Gameplay/BPC_Door.BPC_Door_C") _returnvalue)
  (`self.K2_EndAbility`))

(fn `K2_CanActivateAbility`
  (params (ActorInfo :type "GameplayAbilityActorInfo Structure") (Handle :type "GameplayAbilitySpecHandle Structure"))
  (returns (RelevantTags :type "GameplayTagContainer Structure") (ReturnValue :type Boolean))
  (`parent.K2_CanActivateAbility` ActorInfo Handle)
  (return (struct) (`KismetSystemLibrary.IsValid` (`/Game/Gameplay/Abilities/BFL_ClosestSearches.Get Closest with Component` (`self.GetAvatarActorFromActorInfo`) "/Game/Gameplay/BP_Door.BP_Door_C" "/Game/Gameplay/BPC_Door.BPC_Door_C"))))