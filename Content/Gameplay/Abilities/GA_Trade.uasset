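; Gameplay ability that opens a trade screen with the closest NPC carrying a seller component.
; Activation is allowed only when such a seller is found.
; It hides that NPC's trade text indicator, passes the seller's offers to a WBP_Trade widget, and switches to UI-only input with a cursor.
; The widget's close request removes it, restores game-only input, hides the cursor and ends the ability.
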(event `self.K2_ActivateAbility`
  (bind _returnvalue (`GameplayStatics.GetPlayerController` 0))
  (bind _returnvalue_2 (`/Game/Gameplay/Abilities/BFL_ClosestSearches.Get Closest with Component` (`self.GetAvatarActorFromActorInfo`) "/Game/Gameplay/NPCs/BP_Npc_Base.BP_Npc_Base_C" "/Game/Gameplay/NPCs/BPC_Seller.BPC_Seller_C"))
  (`parent.K2_ActivateAbility`)
  (`SceneComponent.SetVisibility` (`/Game/Gameplay/NPCs/BP_Npc_Base.TradeTextIndicator` (cast `/Game/Gameplay/NPCs/BP_Npc_Base` _returnvalue_2 :!pure true)) false false)
  (bind _returnvalue_3 (`|CreateWidget` "/Game/UI/Trade/WBP_Trade.WBP_Trade_C" (`GameplayStatics.GetPlayerController` 0) (`/Game/Gameplay/NPCs/BPC_Seller.Offers` (`Actor.GetComponentByClass` _returnvalue_2 "/Game/Gameplay/NPCs/BPC_Seller.BPC_Seller_C"))))
  (add `/Game/UI/Trade/WBP_Trade.OnCloseRequest` _returnvalue_3 (delegate `OnCloseRequest_Event`))
  (`UserWidget.AddToViewport` _returnvalue_3 0)
  (`WidgetBlueprintLibrary.SetInputMode_UIOnlyEx` _returnvalue _returnvalue_3)
  (set `PlayerController.bShowMouseCursor` true _returnvalue))

(event `OnCloseRequest_Event`
  (bind _returnvalue (`GameplayStatics.GetPlayerController` 0))
  (`Widget.RemoveFromParent` (stale `self.K2_ActivateAbility` _returnvalue_3))
  (`WidgetBlueprintLibrary.SetInputMode_GameOnly` _returnvalue true)
  (set `PlayerController.bShowMouseCursor` false _returnvalue)
  (`self.K2_EndAbility`))

(fn `K2_CanActivateAbility`
  (params (ActorInfo :type "GameplayAbilityActorInfo Structure") (Handle :type "GameplayAbilitySpecHandle Structure"))
  (returns (RelevantTags :type "GameplayTagContainer Structure") (ReturnValue :type Boolean))
  (`parent.K2_CanActivateAbility` ActorInfo Handle)
  (return (struct) (`KismetSystemLibrary.IsValid` (`/Game/Gameplay/Abilities/BFL_ClosestSearches.Get Closest with Component` (`self.GetAvatarActorFromActorInfo`) "/Game/Gameplay/NPCs/BP_Npc_Base.BP_Npc_Base_C" "/Game/Gameplay/NPCs/BPC_Seller.BPC_Seller_C"))))