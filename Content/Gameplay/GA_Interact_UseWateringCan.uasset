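; Gameplay ability for the watering can interaction that waters the grow spot nearest the avatar.
; Activation requires the parent check to pass and the avatar's BPC_Carrier to hold a BP_Carrieable_WateringCan.
; On interact start, it scans every BP_GrowSpot actor by squared distance and calls PourWater on the closest one's BPC_GrowSpot component, with no range limit.
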(event `self.StartInteract`
  (params (Interactable :type "InteractableComponent Object Reference"))
  (`parent.StartInteract` Interactable)
  (set `self.ClosestGrowSpot` null)
  (set `self.ClosestDist` 999999999999999.0)
  (bind _outactors (`GameplayStatics.GetAllActorsOfClass` "/Game/Gameplay/BP_GrowSpot.BP_GrowSpot_C"))
  (for _array_element _outactors
    (bind _returnvalue (`KismetMathLibrary.Vector_DistanceSquared` (`Actor.K2_GetActorLocation` _array_element) (`Actor.K2_GetActorLocation` (`self.GetAvatarActorFromActorInfo`))))
    (if (< _returnvalue (`self.ClosestDist`))
      (set `self.ClosestGrowSpot` (`Actor.GetComponentByClass` _array_element "/Game/Gameplay/BPC_GrowSpot.BPC_GrowSpot_C"))
      (set `self.ClosestDist` _returnvalue)))
  (`/Game/Gameplay/BPC_GrowSpot.PourWater` (`self.ClosestGrowSpot`)))

(fn `K2_CanActivateAbility`
  (params (ActorInfo :type "GameplayAbilityActorInfo Structure") (Handle :type "GameplayAbilitySpecHandle Structure"))
  (returns (RelevantTags :type "GameplayTagContainer Structure") (ReturnValue :type Boolean))
  (bind _returnvalue (`Actor.GetComponentByClass` (`self.GetAvatarActorFromActorInfo`) "/Game/Gameplay/BPC_Carrier.BPC_Carrier_C"))
  (bind (_relevanttags _returnvalue_2) (`parent.K2_CanActivateAbility` ActorInfo Handle))
  (`/Engine/EditorBlueprintResources/StandardMacros.IsValid` _returnvalue
    (:`Is Valid`
      (if (and (`.bFound` (`/Game/Gameplay/BPC_Carrier.TryGetCurrentCarrieableFiltered` _returnvalue "/Game/Gameplay/BP_Carrieable_WateringCan.BP_Carrieable_WateringCan_C")) _returnvalue_2)
        (return _relevanttags true)
        (else
          _)))
    (:`Is Not Valid`
      _))
  (return _relevanttags false))