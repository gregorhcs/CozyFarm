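; Door component that moves a given actor between an inside and an outside location.
; ToggleInside flips the Inside flag, then sets the passed actor's transform, without sweep, to that of the matching Inside or Outside reference actor.
; The flag is held on the door rather than per actor, so each call alternates the destination regardless of which actor is passed.
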(fn `ToggleInside`
  (params (Actor :type "Actor Object Reference"))
  (if (`self.bInside`)
    (set `self.bInside` false)
    (else
      (set `self.bInside` true)))
  (`Actor.K2_SetActorTransform` Actor (`KismetMathLibrary.SelectTransform` (`Actor.GetTransform` (`self.Inside`)) (`Actor.GetTransform` (`self.Outside`)) (`self.bInside`)) false false))