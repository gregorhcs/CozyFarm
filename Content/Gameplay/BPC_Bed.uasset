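; Bed component that lets the player sleep, skipping in-game time and playing a fade transition.
; Sleep advances the game mode's BPC_InGameTime by HoursToSleep, then calls Fade.
; Fade disables player input, fades the camera to black and back, restores input as the fade-in starts, and briefly shows a WBP_Slept widget.
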(event `Fade`
  (`Actor.DisableInput` (`GameplayStatics.GetPlayerCharacter` 0) (`GameplayStatics.GetPlayerController` 0))
  (`PlayerCameraManager.StartCameraFade` :`self` (`GameplayStatics.GetPlayerCameraManager` 0) :`ToAlpha` 1.0 :`Duration` 1.0 :`bHoldWhenFinished` true)
  (`KismetSystemLibrary.RetriggerableDelay` 2.0)
  (`PlayerCameraManager.StartCameraFade` :`self` (`GameplayStatics.GetPlayerCameraManager` 0) :`FromAlpha` 1.0 :`Duration` 2.0)
  (`Actor.EnableInput` (`GameplayStatics.GetPlayerCharacter` 0) (`GameplayStatics.GetPlayerController` 0))
  (bind _returnvalue (`|CreateWidget` "/Game/UI/WBP_Slept.WBP_Slept_C" (`GameplayStatics.GetPlayerController` 0)))
  (`UserWidget.AddToViewport` _returnvalue 0)
  (`KismetSystemLibrary.RetriggerableDelay` 4.0)
  (`Widget.RemoveFromParent` _returnvalue))

(fn `Sleep`
  (`/Game/Gameplay/BPC_InGameTime.ProgressTime` (`Actor.GetComponentByClass` (`GameplayStatics.GetGameMode`) "/Game/Gameplay/BPC_InGameTime.BPC_InGameTime_C") (`self.HoursToSleep`))
  (`self.Fade`))