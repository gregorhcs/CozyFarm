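; Grow spot component that runs one plant's life cycle of timed growth, watering and harvest.
; Its injected plant tag looks up mesh and growth-stage transforms in PlantData.
; BPC_InGameTime hour events step the plant through those transforms at GrowthFrequency intervals, activating harvest VFX at the last stage.
; Watering shortens the interval after a cooldown shown in text, while Harvest moves the mesh far below and returns its tag.
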(event `self.ReceiveBeginPlay`
  (bind _returnvalue (`Actor.GetComponentByClass` (`GameplayStatics.GetGameMode`) "/Game/Gameplay/BPC_InGameTime.BPC_InGameTime_C"))
  (add `/Game/Gameplay/BPC_InGameTime.NewHour` _returnvalue (delegate `GrowPlant`))
  (add `/Game/Gameplay/BPC_InGameTime.NewHour` _returnvalue (delegate `UpdateCanBeWatered`))
  (`KismetSystemLibrary.DelayUntilNextTick`)
  (`self.UpdateGrowthFrequencyText`)
  (`SceneComponent.K2_SetRelativeTransform` (`self.Plant Component`) (`|GetArrayItem` (`self.GrowthStages`)) false false))

(event `UpdateCanBeWatered`
  (params (Hour :type Integer))
  (set `self.StepsSinceWatered` (- Hour (`self.LastTimeWatered`)))
  (`TextRenderComponent.K2_SetText` (`self.Can be Watered Text`) (`KismetMathLibrary.SelectText` "" (`|FormatText` "Waterable in {n}!" (+ (- (`self.TimeToWaitUntilWateringReady`) (`self.StepsSinceWatered`)) 1)) (< (`self.TimeToWaitUntilWateringReady`) (`self.StepsSinceWatered`)))))

(event `GrowPlant`
  (params (Hour :type Integer))
  (if (== (mod Hour (`self.GrowthFrequency`)) 0)
    (`self.Plant Component`
      (:`then`
        (`self.UpdateGrowthStage`))
      (:`else`))))

(fn `Harvest`
  (returns (`Plant Tag` :type "GameplayTag Structure"))
  (if (`self.bNotHarvested`)
    (`SceneComponent.K2_SetRelativeTransform` (`self.Plant Component`) (`KismetMathLibrary.MakeTransform` (0.0 0.0 -100000.0)) false false)
    (`self.Deactivate` (`self.Harvestable VFX`))
    (`TextRenderComponent.K2_SetText` (`self.Can be Watered Text`) "")
    (`TextRenderComponent.K2_SetText` (`self.Growth Frequency Text`) "Plant harvested!")
    (set `self.bNotHarvested` false)
    (return (`self.Plant Tag`))))

(fn `InjectDependencies`
  (params (PlantComponent :type "StaticMeshComponent Object Reference") (CanBeWateredText :type "TextRenderComponent Object Reference") (GrowthFrequencyText :type "TextRenderComponent Object Reference") (PlantTag :type "GameplayTag Structure") (HarvestableVFX :type "NiagaraComponent Object Reference"))
  (bind _growthstages (`self.GrowthStages`))
  (bind _value (`BlueprintMapLibrary.Map_Find` (`/Game/Gameplay/BP_PlantData.Data` (`self.PlantData`)) PlantTag))
  (set `self.Plant Component` PlantComponent)
  (set `self.Can be Watered Text` CanBeWateredText)
  (set `self.Growth Frequency Text` GrowthFrequencyText)
  (set `self.Harvestable VFX` HarvestableVFX)
  (set `self.Plant Tag` PlantTag)
  (`KismetArrayLibrary.Array_Clear` _growthstages)
  (`KismetArrayLibrary.Array_Append` _growthstages (`.GrowthStages_13_1D3CA73B47E6122243BD61BB8656476B` (break `/Game/Gameplay/F_PlantTemplate` _value)))
  (`StaticMeshComponent.SetStaticMesh` (`self.Plant Component`) (`.Mesh_12_513411F242B7BD69C220EA910D9208B3` (break `/Game/Gameplay/F_PlantTemplate` _value))))

(fn `IsReadyForHarvest`
  (returns (ReturnValue :type Boolean))
  (return (== (`KismetArrayLibrary.Array_Length` (`self.GrowthStages`)) (`self.CurrentGrowthStage`))))

(fn `PourWater`
  (bind _time (`/Game/Gameplay/BPC_InGameTime.CurrentTime` (`Actor.GetComponentByClass` (`GameplayStatics.GetGameMode`) "/Game/Gameplay/BPC_InGameTime.BPC_InGameTime_C")))
  (if (`self.bNotHarvested`)
    (if (< (`self.TimeToWaitUntilWateringReady`) (`self.StepsSinceWatered`))
      (if (> (`self.GrowthFrequency`) 1)
        (`/Engine/EditorBlueprintResources/StandardMacros.DecrementInt` (`self.GrowthFrequency`)
          (:`  `
            (`self.UpdateGrowthFrequencyText`)
            (set `self.LastTimeWatered` _time)
            (`self.UpdateCanBeWatered` _time))))
      (`KismetSystemLibrary.PrintString` "Watered the plant!" true true (struct :`G` 1.0 :`B` 0.040543 :`A` 1.0))
      (else
        (`KismetSystemLibrary.PrintString` "Can't be watered, you just did that!" true true (struct :`G` 1.0 :`B` 0.040543 :`A` 1.0))))))

(fn `SetHarvestable`
  (set `self.CurrentGrowthStage` (`KismetArrayLibrary.Array_LastIndex` (`self.GrowthStages`)))
  (`self.UpdateGrowthStage`))

(fn `UpdateGrowthFrequencyText`
  (`TextRenderComponent.K2_SetText` (`self.Growth Frequency Text`) (`|FormatText` "Growth: 1 / {n} steps" (`self.GrowthFrequency`))))

(fn `UpdateGrowthStage`
  (if (`self.bNotHarvested`)
    (if (!= (`KismetArrayLibrary.Array_Length` (`self.GrowthStages`)) (`self.CurrentGrowthStage`))
      (`SceneComponent.K2_SetRelativeTransform` (`self.Plant Component`) (`|GetArrayItem` (`self.GrowthStages`) (`self.CurrentGrowthStage`)) false false)
      (`/Engine/EditorBlueprintResources/StandardMacros.IncrementInt` (`self.CurrentGrowthStage`)
        (:`  `
          (if (== (`KismetArrayLibrary.Array_Length` (`self.GrowthStages`)) (`self.CurrentGrowthStage`))
            (`self.Activate` (`self.Harvestable VFX`) false)))))))