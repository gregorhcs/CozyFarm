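; Gameplay ability that makes the avatar let go of what it is carrying.
; It can activate only when the parent check passes and the avatar has a valid BPC_Carrier component that is currently carrying.
; On activation it calls LetGo on that component, with no EndAbility call in this graph.
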(event `self.K2_ActivateAbility`
  (`/Game/Gameplay/BPC_Carrier.LetGo` (`Actor.GetComponentByClass` (`self.GetAvatarActorFromActorInfo`) "/Game/Gameplay/BPC_Carrier.BPC_Carrier_C") false))

(fn `K2_CanActivateAbility`
  (params (ActorInfo :type "GameplayAbilityActorInfo Structure") (Handle :type "GameplayAbilitySpecHandle Structure"))
  (returns (RelevantTags :type "GameplayTagContainer Structure") (ReturnValue :type Boolean))
  (bind _returnvalue (`Actor.GetComponentByClass` (`self.GetAvatarActorFromActorInfo`) "/Game/Gameplay/BPC_Carrier.BPC_Carrier_C"))
  (bind (_relevanttags _returnvalue_2) (`parent.K2_CanActivateAbility` ActorInfo Handle))
  (`/Engine/EditorBlueprintResources/StandardMacros.IsValid` _returnvalue
    (:`Is Valid`
      (return _relevanttags (and (`/Game/Gameplay/BPC_Carrier.IsCarrying` _returnvalue) _returnvalue_2)))
    (:`Is Not Valid`
      (return _relevanttags false))))