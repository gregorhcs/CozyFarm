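; Gameplay ability for the watering can interaction, which waters the nearest grow spot.
; Activation requires the avatar's BPC_Carrier to hold a BP_Carrieable_WateringCan; the parent check is called, but its boolean result is ignored.
; On activation it finds the closest actor with a BPC_GrowSpot, calls PourWater on that component without a validity check and ends immediately.
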(event `self.K2_ActivateAbility`
  (`/Game/Gameplay/BPC_GrowSpot.PourWater` (`Actor.GetComponentByClass` (`/Game/Gameplay/New/BFL_ClosestSearches.Get Closest Actor with Component` (`self.GetAvatarActorFromActorInfo`) "/Game/Gameplay/BPC_GrowSpot.BPC_GrowSpot_C") "/Game/Gameplay/BPC_GrowSpot.BPC_GrowSpot_C"))
  (`self.K2_EndAbility`))

(fn `K2_CanActivateAbility`
  (params (ActorInfo :type "GameplayAbilityActorInfo Structure") (Handle :type "GameplayAbilitySpecHandle Structure"))
  (returns (RelevantTags :type "GameplayTagContainer Structure") (ReturnValue :type Boolean))
  (bind _returnvalue (`Actor.GetComponentByClass` (`self.GetAvatarActorFromActorInfo`) "/Game/Gameplay/BPC_Carrier.BPC_Carrier_C"))
  (bind _relevanttags (`parent.K2_CanActivateAbility` ActorInfo Handle))
  (`/Engine/EditorBlueprintResources/StandardMacros.IsValid` _returnvalue
    (:`Is Valid`
      (return _relevanttags (`.bFound` (`/Game/Gameplay/BPC_Carrier.TryGetCurrentCarrieableFiltered` _returnvalue "/Game/Gameplay/BP_Carrieable_WateringCan.BP_Carrieable_WateringCan_C"))))
    (:`Is Not Valid`
      (return (struct) false))))