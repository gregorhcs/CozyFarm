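; Gameplay Ability for sprinting that raises the avatar's CharacterMovement max walk speed while the input is held.
; After a successful commit, a fast looping timer checks velocity and sets IsSprinting when the avatar moves above normal speed.
; Releasing input ends the ability, which restores walk speed, clears the timer and resets the flag.
; Despite the CheckForStaminaUse name, the graph itself applies no stamina drain.
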(event `self.K2_OnEndAbility`
  (params (bWasCancelled :type Boolean))
  (set `CharacterMovementComponent.MaxWalkSpeed` 300.0 (`self.CharacterMovement`))
  (`KismetSystemLibrary.K2_ClearAndInvalidateTimerHandle` (`self.SprintStartDelayTimer`))
  (set `self.bIsSprinting` false))

(event `self.K2_ActivateAbility`
  (bind _returnvalue (`self.K2_CommitAbility`))
  (if _returnvalue
    (set `self.CharacterMovement` (`Actor.GetComponentByClass` (`self.GetAvatarActorFromActorInfo`) "/Script/Engine.CharacterMovementComponent"))
    (set `CharacterMovementComponent.MaxWalkSpeed` 600.0 (`self.CharacterMovement`))
    (bind _returnvalue_2 (`KismetSystemLibrary.K2_SetTimerDelegate` (delegate `CheckForStaminaUse`) 0.05 true))
    (set `self.SprintStartDelayTimer` _returnvalue_2)
    (`AbilityTask_WaitInputRelease.WaitInputRelease` false
      (:`OnRelease`
        (`self.K2_EndAbility`)))
    (else
      (`self.K2_CancelAbility`))))

(event `CheckForStaminaUse`
  (if (> (`KismetMathLibrary.VSize` (`CharacterMovementComponent.GetLastUpdateVelocity` (`self.CharacterMovement`))) 300.0)
    (if (not (`self.bIsSprinting`))
      (set `self.bIsSprinting` true))
    (else
      (set `self.bIsSprinting` false))))