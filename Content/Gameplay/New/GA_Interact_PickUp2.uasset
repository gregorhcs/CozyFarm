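; Gameplay ability that makes player character 0 pick up the closest actor with a carrieable component.
; On activation, it passes that actor's BPC_Carrieable to the player's BPC_Carrier PickUp, then ends immediately.
; Activation is allowed only if the carrier exists and is not already carrying, ignoring the parent check's boolean result.
; It always targets player index 0 rather than the ability's owner.
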(event `self.K2_ActivateAbility`
  (`parent.K2_ActivateAbility`)
  (`/Game/Gameplay/BPC_Carrier.PickUp` (`Actor.GetComponentByClass` (`GameplayStatics.GetPlayerCharacter` 0) "/Game/Gameplay/BPC_Carrier.BPC_Carrier_C") (`Actor.GetComponentByClass` (`/Game/Gameplay/New/BFL_ClosestSearches.Get Closest Actor with Component` (`GameplayStatics.GetPlayerCharacter` 0) "/Game/Gameplay/BPC_Carrieable.BPC_Carrieable_C") "/Game/Gameplay/BPC_Carrieable.BPC_Carrieable_C"))
  (`self.K2_EndAbility`))

(fn `K2_CanActivateAbility`
  (params (ActorInfo :type "GameplayAbilityActorInfo Structure") (Handle :type "GameplayAbilitySpecHandle Structure"))
  (returns (RelevantTags :type "GameplayTagContainer Structure") (ReturnValue :type Boolean))
  (bind _returnvalue (`Actor.GetComponentByClass` (`GameplayStatics.GetPlayerCharacter` 0) "/Game/Gameplay/BPC_Carrier.BPC_Carrier_C"))
  (bind _relevanttags (`parent.K2_CanActivateAbility` ActorInfo Handle))
  (`/Engine/EditorBlueprintResources/StandardMacros.IsValid` _returnvalue
    (:`Is Valid`
      (return _relevanttags (not (`/Game/Gameplay/BPC_Carrier.IsCarrying` _returnvalue))))
    (:`Is Not Valid`
      (return _relevanttags false))))