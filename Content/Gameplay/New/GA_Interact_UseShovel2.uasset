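; Gameplay ability that lets a character carrying a shovel place a grow spot on the ground beneath them.
; Activation is allowed only when the avatar's carrier component reports a held shovel carrieable.
; On activation it traces downward from the avatar, spawns a BP_GrowSpot at the hit location, then ends the ability whether or not anything was hit.
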(event `self.K2_ActivateAbility`
  (bind _returnvalue (`self.GetAvatarActorFromActorInfo`))
  (bind _returnvalue_2 (`Actor.K2_GetActorLocation` _returnvalue))
  (bind (_outhit _returnvalue_3) (`KismetSystemLibrary.LineTraceSingle` _returnvalue_2 (- _returnvalue_2 (0.0 0.0 1000.0)) "TraceTypeQuery1" true (`|MakeArray` _returnvalue)))
  (if _returnvalue_3
    (`|SpawnActorFromClass` "/Game/Gameplay/BP_GrowSpot.BP_GrowSpot_C" (`KismetMathLibrary.MakeTransform` (`.Location` (`GameplayStatics.BreakHitResult` _outhit))) "Undefined" "MultiplyWithRoot" null null)
    (`self.K2_EndAbility`)
    (else
      (`self.K2_EndAbility`))))

(fn `K2_CanActivateAbility`
  (params (ActorInfo :type "GameplayAbilityActorInfo Structure") (Handle :type "GameplayAbilitySpecHandle Structure"))
  (returns (RelevantTags :type "GameplayTagContainer Structure") (ReturnValue :type Boolean))
  (bind _returnvalue (`Actor.GetComponentByClass` (`self.GetAvatarActorFromActorInfo`) "/Game/Gameplay/BPC_Carrier.BPC_Carrier_C"))
  (bind _relevanttags (`parent.K2_CanActivateAbility` ActorInfo Handle))
  (`/Engine/EditorBlueprintResources/StandardMacros.IsValid` _returnvalue
    (:`Is Valid`
      (return _relevanttags (`.bFound` (`/Game/Gameplay/BPC_Carrier.TryGetCurrentCarrieableFiltered` _returnvalue "/Game/Gameplay/BP_Carrieable_Shovel.BP_Carrieable_Shovel_C"))))
    (:`Is Not Valid`
      (return (struct) false))))