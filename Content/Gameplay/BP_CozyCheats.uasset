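; BP_CozyCheats holds debug cheat functions for testing the game's economy, clock and NPCs.
; Money, seed and plant cheats add fixed amounts to the player's BPC_Inventory, covering every key in PlantData.
; Time cheats progress the game mode's BPC_InGameTime by preset steps.
; The teleport cheat cycles through BP_Npc_Base actors, moving the player to a random navigable point near each one, raised slightly above the ground.
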(fn `CZ_AddMoney100`
  (`/Game/Gameplay/BPC_Inventory.AddMoney` (`Actor.GetComponentByClass` (`GameplayStatics.GetPlayerCharacter` 0) "/Game/Gameplay/BPC_Inventory.BPC_Inventory_C") 100))

(fn `CZ_AddPlantsOfEachKind10`
  (bind _keys (`BlueprintMapLibrary.Map_Keys` (`/Game/Gameplay/BP_PlantData.Data` (`self.PlantData`))))
  (for _array_element _keys
    (`/Game/Gameplay/BPC_Inventory.AddPlants` (`Actor.GetComponentByClass` (`GameplayStatics.GetPlayerCharacter` 0) "/Game/Gameplay/BPC_Inventory.BPC_Inventory_C") _array_element 10)))

(fn `CZ_AddSeedsOfEachKind10`
  (bind _keys (`BlueprintMapLibrary.Map_Keys` (`/Game/Gameplay/BP_PlantData.Data` (`self.PlantData`))))
  (for _array_element _keys
    (`/Game/Gameplay/BPC_Inventory.AddSeeds` (`Actor.GetComponentByClass` (`GameplayStatics.GetPlayerCharacter` 0) "/Game/Gameplay/BPC_Inventory.BPC_Inventory_C") _array_element 10)))

(fn `CZ_AdvanceTimeBy1`
  (`/Game/Gameplay/BPC_InGameTime.ProgressTime` (`Actor.GetComponentByClass` (`GameplayStatics.GetGameMode`) "/Game/Gameplay/BPC_InGameTime.BPC_InGameTime_C") 1))

(fn `CZ_AdvanceTimeBy10`
  (`/Game/Gameplay/BPC_InGameTime.ProgressTime` (`Actor.GetComponentByClass` (`GameplayStatics.GetGameMode`) "/Game/Gameplay/BPC_InGameTime.BPC_InGameTime_C") 10))

(fn `CZ_AdvanceTimeBy5`
  (`/Game/Gameplay/BPC_InGameTime.ProgressTime` (`Actor.GetComponentByClass` (`GameplayStatics.GetGameMode`) "/Game/Gameplay/BPC_InGameTime.BPC_InGameTime_C") 5))

(fn `CZ_TeleportToNextCharacter`
  (bind _outactors (`GameplayStatics.GetAllActorsOfClass` "/Game/Gameplay/NPCs/BP_Npc_Base.BP_Npc_Base_C"))
  (set `self.Characters` _outactors)
  (bind _result (`/Engine/EditorBlueprintResources/StandardMacros.IncrementInt` (`self.CharacterIndex`))
    (:`  `
      (if (> _result (`KismetArrayLibrary.Array_LastIndex` (`self.Characters`)))
        (set `self.CharacterIndex` 0))
      (bind _randomlocation (`NavigationSystemV1.K2_GetRandomLocationInNavigableRadius` (`Actor.K2_GetActorLocation` (`|GetArrayItem` (`self.Characters`) (`self.CharacterIndex`))) 300.0 null "/Script/AIModule.NavFilter_AIControllerDefault"))
      (`Actor.K2_SetActorLocation` (`GameplayStatics.GetPlayerCharacter` 0) (+ _randomlocation (0.0 0.0 100.0)) false false))))